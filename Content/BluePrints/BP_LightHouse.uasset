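; BP_LightHouse is a light actor whose point light responds to the player character entering or leaving its Box trigger.
; Begin and end overlap events filter for BP_ThirdPersonCharacter, then each restarts its own timeline from the start.
; The On and Off timeline curves drive a lerp between zero and the Intensity variable, setting the point light's brightness on each update.
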(event OnComponentEndOverlap(Box)
  (params (OverlappedComponent :type Primitive%20Component%20Object%20Reference) (OtherActor :type Actor%20Object%20Reference) (OtherComp :type Primitive%20Component%20Object%20Reference) (OtherBodyIndex :type Integer))
  (Utilities|Casting|CastToBP_ThirdPersonCharacter OtherActor)
  (bind _off (Timeline|Timeline PlayFromStart)
    (:Update
      (Rendering|Components|Light|SetIntensity (Variables|Default|GetPointLightComponent) (Math|Float|Lerp 0.0 (Variables|Default|GetIntensity) _off)))))

(event OnComponentBeginOverlap(Box)
  (params (OverlappedComponent :type Primitive%20Component%20Object%20Reference) (OtherActor :type Actor%20Object%20Reference) (OtherComp :type Primitive%20Component%20Object%20Reference) (OtherBodyIndex :type Integer) (bFromSweep :type Boolean) (SweepResult :type Hit%20Result%20Structure%20%28by%20ref%29))
  (Utilities|Casting|CastToBP_ThirdPersonCharacter OtherActor)
  (bind _on (Timeline|On PlayFromStart)
    (:Update
      (Rendering|Components|Light|SetIntensity (Variables|Default|GetPointLightComponent) (Math|Float|Lerp 0.0 (Variables|Default|GetIntensity) _on)))))

(fn ConstructionScript)